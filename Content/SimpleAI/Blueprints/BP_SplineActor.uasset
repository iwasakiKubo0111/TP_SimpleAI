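; BP_SplineActor renders a routing tube along a spline, likely to visualize a path for the SimpleAI content.
; The construction script aligns the spline to the scene root, then adds one Z-forward SplineMeshComponent per segment, using SM_RoutingTube and that segment's endpoint locations and tangents.
; BeginPlay prints the Location variable and moves spline point 1 there, without rebuilding the meshes.
; Destroyed only prints a debug string.
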(event EventBeginPlay
  (bind _location (Variables|Default|GetLocation))
  (Development|PrintString (Utilities|String|ToString(Vector) _location))
  (Spline|SetLocationatSplinePoint (Variables|Default|GetSpline) 1 _location "Local" true))

(event Collision|EventActorBeginOverlap
  (params (OtherActor :type Actor%20Object%20Reference)))

(event EventTick
  (params (DeltaSeconds :type Float%20%28single-precision%29)))

(event EventDestroyed
  (Development|PrintString "destryed"))

(fn ConstructionScript
  (bind _spline (Variables|Default|GetSpline))
  (Transformation|SetWorldTransform (Variables|Default|GetSpline) (Transformation|GetWorldTransform (Variables|Default|GetDefaultSceneRoot)) false false)
  ;[1 1 1] セグメント数分実行
  (for _index (range 0 (- (Class|SplineComponent|GetNumberOfSplineSegments (Variables|Default|GetSpline)) 1))
    (bind _returnvalue (AddComponent|AddSplineMeshComponent false))
    (Transformation|AttachComponentToComponent _returnvalue (Variables|Default|GetSpline) "None" "KeepRelative" "KeepRelative" "KeepRelative" true)
    (SplineMesh|SetForwardAxis _returnvalue "Z" true)
    (Components|StaticMesh|SetStaticMesh _returnvalue "/Game/SimpleAI/SM/SM_RoutingTube.SM_RoutingTube")
    (SplineMesh|SetStartandEnd _returnvalue (.Location (Spline|GetLocationandTangentatSplinePoint _spline _index "Local")) (.Tangent (Spline|GetLocationandTangentatSplinePoint _spline _index "Local")) (.Location (Spline|GetLocationandTangentatSplinePoint _spline (+ _index 1) "Local")) (.Tangent (Spline|GetLocationandTangentatSplinePoint _spline (+ _index 1) "Local")) true :!class /Script/Engine.SplineMeshComponent)))